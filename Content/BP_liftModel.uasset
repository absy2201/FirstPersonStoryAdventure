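; Lift car actor with a sliding door that carries the player between two heights.
; Trigger boxes track the player inside and toggle BP_liftButton clickability; leaving the car auto-closes the door after a delay.
; Timeline lerps drive door and car, with flags blocking travel during door motion and Box1 collision sealing the closed doorway.
; Arrival opens the door and re-enables the button; older gate and DoOnce logic remains disconnected.
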(event OnComponentBeginOverlap(Box)
  (params (OverlappedComponent :type Primitive%20Component%20Object%20Reference) (OtherActor :type Actor%20Object%20Reference) (OtherComp :type Primitive%20Component%20Object%20Reference) (OtherBodyIndex :type Integer) (bFromSweep :type Boolean) (SweepResult :type Hit%20Result%20Structure%20%28by%20ref%29))
  (Variables|Default|SetisPlayerIn? true)
  (Development|PrintString "player in"))

(event OnComponentEndOverlap(Box)
  (params (OverlappedComponent :type Primitive%20Component%20Object%20Reference) (OtherActor :type Actor%20Object%20Reference) (OtherComp :type Primitive%20Component%20Object%20Reference) (OtherBodyIndex :type Integer))
  (Variables|Default|SetisPlayerIn? false)
  (Development|PrintString "player out")
  (Variables|Default|SetcanAutoCloseDoor? true)
  (Utilities|FlowControl|Delay 1.0)
  (CallFunction|CloseDoorFunc))

(event OnComponentBeginOverlap(Box_buttonCanClick)
  (params (OverlappedComponent :type Primitive%20Component%20Object%20Reference) (OtherActor :type Actor%20Object%20Reference) (OtherComp :type Primitive%20Component%20Object%20Reference) (OtherBodyIndex :type Integer) (bFromSweep :type Boolean) (SweepResult :type Hit%20Result%20Structure%20%28by%20ref%29))
  (bind _outactors (Actor|GetAllActorsOfClass "/Game/StoryAdvTemplate/BP_liftButton.BP_liftButton_C"))
  (bind _asbp_lift_button (Utilities|Casting|CastToBP_liftButton (Utilities|Array|Get(acopy) _outactors)))
  (Variables|/Game/StoryAdvTemplate/BP_liftButton.BP_liftButton_C|SetcanBeClicked? _asbp_lift_button true))

(event OnComponentEndOverlap(Box_buttonCanClick)
  (params (OverlappedComponent :type Primitive%20Component%20Object%20Reference) (OtherActor :type Actor%20Object%20Reference) (OtherComp :type Primitive%20Component%20Object%20Reference) (OtherBodyIndex :type Integer))
  (bind _outactors (Actor|GetAllActorsOfClass "/Game/StoryAdvTemplate/BP_liftButton.BP_liftButton_C"))
  (bind _asbp_lift_button (Utilities|Casting|CastToBP_liftButton (Utilities|Array|Get(acopy) _outactors)))
  (Variables|/Game/StoryAdvTemplate/BP_liftButton.BP_liftButton_C|SetcanBeClicked? _asbp_lift_button false))

(event Custom|OpenDoorFunc
  (bind _doorstartpos_x (Variables|Default|GetDoorStartPos_X))
  (if (Variables|Default|GetcanOpenDoor?)
    (if (not (and (Variables|Default|GetisGoingUp?) (Variables|Default|GetisGoingDown?)))
      (Variables|Default|SetcanOpenDoor? false)
      (Collision|SetCollisionEnabled (Variables|Default|GetBox1) "NoCollision")
      (Variables|Default|SetcanLiftMove? false)
      (bind _newtrack_0 (Timeline|Timeline_5 PlayFromStart)
        (:Update
          (Transformation|SetRelativeLocation (Variables|Default|Getmesh_door) (Math|Vector|MakeVector (Math|Float|Lerp _doorstartpos_x (+ _doorstartpos_x 2.3e+02) _newtrack_0) (Variables|Default|GetDoorOriginalPos_Y) (Variables|Default|GetDoorOriginalPos_Z)) false false))
        (:Finished
          (Variables|Default|SetcanLiftMove? true)
          (Variables|Default|SetcanCloseDoor? true)
          (Variables|Default|SetisDoorOpen? true))))))

(event Custom|CloseDoorFunc
  (bind _doorstartpos_x (Variables|Default|GetDoorStartPos_X))
  (if (Variables|Default|GetcanCloseDoor?)
    (if (not (and (Variables|Default|GetisGoingUp?) (Variables|Default|GetisGoingDown?)))
      (Variables|Default|SetcanCloseDoor? false)
      (Collision|SetCollisionEnabled (Variables|Default|GetBox1) "QueryAndPhysics")
      (Variables|Default|SetcanLiftMove? false)
      (bind _newtrack_0 (Timeline|Timeline_6 PlayFromStart)
        (:Update
          (Transformation|SetRelativeLocation (Variables|Default|Getmesh_door) (Math|Vector|MakeVector (Math|Float|Lerp (+ _doorstartpos_x 2.3e+02) _doorstartpos_x _newtrack_0) (Variables|Default|GetDoorOriginalPos_Y) (Variables|Default|GetDoorOriginalPos_Z)) false false))
        (:Finished
          (Variables|Default|SetcanLiftMove? true)
          (Variables|Default|SetcanOpenDoor? true)
          (Variables|Default|SetisDoorOpen? false))))))

(event Custom|LiftGoDown
  (if (and (Variables|Default|GetcanLiftMove?) (Variables|Default|GetisPlayerIn?))
    (bind _newtrack_0 (Timeline|Timeline_7 Play)
      (:Update
        (Transformation|SetWorldLocation (Variables|Default|GetDefaultSceneRoot) (Math|Vector|MakeVector (Variables|Default|GetoriginXpos) (Variables|Default|GetoriginYpos) (Math|Float|Lerp (Variables|Default|GetendZpos) (Variables|Default|GetstartZpos) _newtrack_0)) false false))
      (:Finished
        (Utilities|FlowControl|Delay 2.0)
        (CallFunction|OpenDoorFunc)
        (Variables|Default|SetcanCloseDoor? false)
        (Variables|Default|SetcanOpenDoor? true)
        (bind _outactors (Actor|GetAllActorsOfClass "/Game/StoryAdvTemplate/BP_liftButton.BP_liftButton_C"))
        (Variables|/Game/StoryAdvTemplate/BP_liftButton.BP_liftButton_C|SetcanBeClicked? (Utilities|Array|Get(acopy) _outactors) true)))))

(event Custom|LiftGoUp
  (if (and (Variables|Default|GetcanLiftMove?) (Variables|Default|GetisPlayerIn?))
    (bind _newtrack_0 (Timeline|Timeline_8 Play)
      (:Update
        (Transformation|SetWorldLocation (Variables|Default|GetDefaultSceneRoot) (Math|Vector|MakeVector (Variables|Default|GetoriginXpos) (Variables|Default|GetoriginYpos) (Math|Float|Lerp (Variables|Default|GetstartZpos) (Variables|Default|GetendZpos) _newtrack_0)) false false))
      (:Finished
        (Utilities|FlowControl|Delay 2.0)
        (CallFunction|OpenDoorFunc)
        (Variables|Default|SetcanCloseDoor? false)
        (Variables|Default|SetcanOpenDoor? true)
        (bind _outactors (Actor|GetAllActorsOfClass "/Game/StoryAdvTemplate/BP_liftButton.BP_liftButton_C"))
        (Variables|/Game/StoryAdvTemplate/BP_liftButton.BP_liftButton_C|SetcanBeClicked? (Utilities|Array|Get(acopy) _outactors) true)))))

(event EventBeginPlay
  (Collision|SetCollisionEnabled (Variables|Default|GetBox1) "NoCollision")
  (Variables|Default|SetcanOpenDoor? true))

(event Collision|EventActorBeginOverlap
  (params (OtherActor :type Actor%20Object%20Reference)))

(event EventTick
  (params (DeltaSeconds :type Float%20%28single-precision%29))
  ;[1 1 1] Wrong way to do this....
)

(event Input|KeyboardEvents|O
  (params (Key :type Key%20Structure :default "None"))
  ;[1 1 1] Only for test
)

(fn ConstructionScript)