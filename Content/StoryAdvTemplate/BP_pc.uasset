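; BP_pc is an interactable object, apparently a PC, that opens a screen UI when the player interacts with it.
; The inherited Interaction event runs only while IsOn is false, disabling input on BP_FirstPersonCharacter and adding a UI_Screen widget to the viewport.
; It then sets IsOn to block repeat opens; nothing here resets the flag or restores input.
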(event EventInteraction
  ;[0 0.7682 1] Inherited Event
  (if (not (Variables|Default|GetisOn?))
    (bind _asbp_first_person_character (Utilities|Casting|CastToBP_FirstPersonCharacter (Game|GetPlayerCharacter 0)))
    (Input|DisableInput _asbp_first_person_character (Game|GetPlayerController 0))
    (bind _returnvalue (UserInterface|CreateWidget "/Game/StoryAdvTemplate/UI_Screen.UI_Screen_C" (Game|GetPlayerController 0)))
    (UserInterface|Viewport|AddtoViewport _returnvalue 0)
    (Variables|Default|SetisOn? true)))

(fn ConstructionScript
  (|CallParentFunction))