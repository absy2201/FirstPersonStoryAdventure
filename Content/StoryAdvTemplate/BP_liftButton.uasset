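; BP_liftButton is an interactable button that closes the lift door and sends the lift down or up.
; Interaction plays a click sound, then proceeds only if CanBeClicked is true and the first BP_liftModel found has its door open.
; It clears CanBeClicked and, given a valid DoorReference, calls CloseDoorFunc after a short delay.
; After a longer delay, a FlipFlop alternates between LiftGoDown and LiftGoUp on that reference.
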(event EventInteraction
  (bind _doorreference (Variables|Default|GetDoorReference))
  ;[0 0.7682 1] Inherited Event
  (Audio|PlaySound2D "/Game/StoryAdvTemplate/PC/Sound/1891_computer-mouse-click-01.1891_computer-mouse-click-01" 1.0 1.0 0.0 0 0)
  (bind _outactors (Actor|GetAllActorsOfClass "/Game/BP_liftModel.BP_liftModel_C"))
  (if (and (Variables|Default|GetcanBeClicked?) (Variables|/Game/BP_liftModel.BP_liftModel_C|GetisDoorOpen? (Utilities|Array|Get(acopy) _outactors)))
    (Variables|Default|SetcanBeClicked? false)
    (Utilities|IsValid _doorreference
      (:Is%20Valid
        (Utilities|FlowControl|Delay 0.5)
        (Default|CloseDoorFunc _doorreference)
        (Utilities|FlowControl|Delay 3.6)
        (Utilities|FlowControl|FlipFlop
          (:A
            (Default|LiftGoDown _doorreference))
          (:B
            (Default|LiftGoUp _doorreference)))))))

(fn ConstructionScript
  (|CallParentFunction))