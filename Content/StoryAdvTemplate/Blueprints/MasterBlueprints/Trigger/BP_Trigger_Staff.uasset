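; BP_Trigger_Staff is a story trigger that plays staff and find-garage-key voice-overs when the player enters it.
; On BeginPlay it disables itself through AllowTrigger and caches the BP_GameController, retrying on a timer until one exists.
; Once AllowTrigger is set from outside this graph, the first player overlap plays StaffVO, waits out its duration plus a pause, then plays FindGarageKeyVO.
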(event Custom|SetInstances
  (bind _outactors (Actor|GetAllActorsOfClass "/Game/StoryAdvTemplate/Blueprints/BP_GameController.BP_GameController_C"))
  (if (Utilities|Array|IsValidIndex _outactors)
    (Variables|Default|SetGameControllerInstance (Utilities|Array|Get(acopy) _outactors))
    (else
      (Utilities|Time|SetTimerbyEvent (delegate Custom|SetInstances) 0.5))))

(event EventBeginPlay
  (CallFunction|SetInstances)
  (Variables|Default|SetallowTrigger false))

(event Collision|EventActorBeginOverlap
  (params (OtherActor :type Actor%20Object%20Reference))
  (bind _staffvo (Variables|Default|GetStaffVO))
  (if (Variables|Default|GetallowTrigger)
    (if (== OtherActor (Game|Player|GetPlayerPawn 0))
      (Utilities|FlowControl|DoOnce false
        (:Completed
          (Utilities|FlowControl|Delay 1.0)
          (Default|PlayVoiceOver (Variables|Default|GetGameControllerInstance) _staffvo)
          (Utilities|FlowControl|Delay (Variables|/Script/Engine.SoundBase|GetDuration _staffvo))
          (Utilities|FlowControl|Delay 2.0)
          (Default|PlayVoiceOver (Variables|Default|GetGameControllerInstance) (Variables|Default|GetFindGarageKeyVO)))))))

(event EventTick
  (params (DeltaSeconds :type Float%20%28single-precision%29)))

(fn ConstructionScript
  (|CallParentFunction))