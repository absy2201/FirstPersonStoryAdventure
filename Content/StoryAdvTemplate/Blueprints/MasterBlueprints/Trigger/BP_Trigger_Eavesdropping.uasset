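; BP_Trigger_Eavesdropping is a story trigger that plays an overheard NPC conversation the first time the player pawn enters it.
; On overlap, a DoOnce plays the NPC dialog at the trigger's location, waits briefly, then plays an eavesdropping voice-over.
; It then sets HasEndGame1 on BP_GameController, which it finds at BeginPlay, retrying on a timer until one exists.
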(event Custom|SetInstances
  (bind _outactors (Actor|GetAllActorsOfClass "/Game/StoryAdvTemplate/Blueprints/BP_GameController.BP_GameController_C"))
  (if (Utilities|Array|IsValidIndex _outactors)
    (Variables|Default|SetGameControllerInstance (Utilities|Array|Get(acopy) _outactors))
    (else
      (Utilities|Time|SetTimerbyEvent (delegate Custom|SetInstances) 0.5))))

(event EventBeginPlay
  (CallFunction|SetInstances))

(event Collision|EventActorBeginOverlap
  (params (OtherActor :type Actor%20Object%20Reference))
  (if (== OtherActor (Game|Player|GetPlayerPawn 0))
    (Utilities|FlowControl|DoOnce false
      (:Completed
        (Audio|SpawnSoundatLocation (Variables|Default|GetNPCDialog) (Transformation|GetActorLocation) "0, 0, 0" 1.0 1.0 0.0 0 0)
        (Utilities|FlowControl|Delay 4.0)
        (Audio|SpawnSoundatLocation (Variables|Default|GetEavesdroppingVO) (Transformation|GetActorLocation) "0, 0, 0" 1.0 1.0 0.0 0 0)
        (Variables|/Game/StoryAdvTemplate/Blueprints/BP_GameController.BP_GameController_C|SethasEndGame1? (Variables|Default|GetGameControllerInstance) true)))))

(event EventTick
  (params (DeltaSeconds :type Float%20%28single-precision%29)))

(fn ConstructionScript
  (|CallParentFunction))