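; BP_Router is an interactable router in the story adventure template that the player switches on.
; Its inherited Interaction event plays a click sound and, if the light is off, shows BottomLight and sets the light and router-on flags.
; It then finds BP_GameController with GetAllActorsOfClass and has it play the router-on voice-over.
; Switching is one-way, as the turn-off logic is never run.
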(event EventInteraction
  ;[0 0.7682 1] Inherited Event
  (Audio|PlaySound2D "/Game/StoryAdvTemplate/PC/Sound/1891_computer-mouse-click-01.1891_computer-mouse-click-01" 1.0 1.0 0.0 0 0)
  ;[0 0.7682 1] Interaction Code: Simple Lamp Functionality (On / Off)
  (if (not (Variables|Default|GetisLightOn?))
    (Rendering|SetVisibility (Variables|Default|GetBottomLight) true false)
    (Variables|Default|SetisLightOn? true)
    (Variables|Default|SetisRouterOn? true)
    (bind _outactors (Actor|GetAllActorsOfClass "/Game/StoryAdvTemplate/Blueprints/BP_GameController.BP_GameController_C"))
    (bind _asbp_game_controller (Utilities|Casting|CastToBP_GameController (Utilities|Array|Get(acopy) _outactors)))
    (Default|PlayVoiceOver _asbp_game_controller (Variables|Default|GetRounterIsOnVO))))

(fn ConstructionScript
  (|CallParentFunction))