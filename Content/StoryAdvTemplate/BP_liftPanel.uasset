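; BP_liftPanel is an interactable lift panel that opens its linked door for a player outside the lift.
; When usable, it plays a click and checks the first BP_liftModel found for player absence and permission to open.
; It then calls OpenDoorFunc on DoorReference, with a DoOnce and delay blocking repeat presses briefly.
; When unusable, it has BP_GameController play a lift-not-working voice-over.
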(event EventInteraction
  (bind _doorreference (Variables|Default|GetDoorReference))
  ;[0 0.7682 1] Inherited Event
  (if (Variables|Default|GetcanUse?)
    (Audio|PlaySound2D "/Game/StoryAdvTemplate/PC/Sound/1891_computer-mouse-click-01.1891_computer-mouse-click-01" 1.0 1.0 0.0 0 0)
    (bind _outactors (Actor|GetAllActorsOfClass "/Game/BP_liftModel.BP_liftModel_C"))
    (if (and (not (Variables|/Game/BP_liftModel.BP_liftModel_C|GetisPlayerIn? (Utilities|Array|Get(acopy) _outactors))) (Variables|/Game/BP_liftModel.BP_liftModel_C|GetcanOpenDoor? (Utilities|Array|Get(acopy) _outactors)))
      (Utilities|IsValid _doorreference
        (:Is%20Valid
          (Utilities|FlowControl|DoOnce false :!label _label
            (:Completed
              (Default|OpenDoorFunc _doorreference)
              (Development|PrintString "door opened!")
              (Utilities|FlowControl|Delay 4.0)
              (goto _label Reset))))))
    (else
      (bind _outactors_2 (Actor|GetAllActorsOfClass "/Game/StoryAdvTemplate/Blueprints/BP_GameController.BP_GameController_C"))
      (Default|PlayVoiceOver (Utilities|Array|Get(acopy) _outactors_2) (Variables|Default|GetLiftNotWorkingVO)))))

(fn ConstructionScript
  (|CallParentFunction))